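; VR player pawn that handles camera-relative movement, snap turning and two-handed grabbing.
; BeginPlay adds the VR input context, corrects VRRoot height to a desired camera height after a delay, and spawns BP_Hand actors attached to VRRoot, with an offset layout in test mode.
; Grab inputs forward to each hand.
; SnapTurn rotates the actor, then offsets it to cancel the resulting camera displacement.
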(event `self.ReceiveBeginPlay`
  (bind _istest (`self.IsTest`))
  (bind (_returnvalue_x _returnvalue_y _returnvalue_z) (`KismetMathLibrary.BreakVector` (`SceneComponent.K2_GetComponentLocation` (`self.Camera`))))
  (`|ExecutionSequence`
    (:`then_0`
      ;[1 1 1] Input Mapping Context
      (`EnhancedInputSubsystemInterface.AddMappingContext` (pcsubsystem `EnhancedInputLocalPlayerSubsystem` (`GameplayStatics.GetPlayerController` 0)) "/Game/BluePrint/Input/IMC_VR_Default.IMC_VR_Default" 0 (struct)))
    (:`then_1`
      ;[1 1 1] 원하는 시작위치로 VRRoot를 보정하여 시작할 수 있어야 한다
      (`HeadMountedDisplayFunctionLibrary.SetTrackingOrigin` "View")
      (`KismetSystemLibrary.Delay` 1.0) ; 물리 시간 보정용 delay
      (`SceneComponent.K2_AddRelativeLocation` (`self.VRRoot`) (`KismetMathLibrary.MakeVector` 0.0 0.0 (- (`self.DesiredCameraHeight`) _returnvalue_z)) false false))
    (:`then_2`
      (if _istest
        (bind _returnvalue (`|SpawnActorFromClass` "/Game/BluePrint/Hand/BP_Hand.BP_Hand_C" (`KismetMathLibrary.MakeTransform` (100.0 0.0 0.0) (struct :`Pitch` 90.0 :`Roll` 90.0)) "AlwaysSpawn" "MultiplyWithRoot" self true null))
        (bind _output_get (set `self.LeftHand` _returnvalue))
        (`self.K2_AttachToComponent` _output_get (`self.VRRoot`) "None" "KeepRelative" "SnapToTarget" "KeepWorld" true)
        (else
          ;[1 1 1] Make Hand
          (bind _returnvalue_2 (`|SpawnActorFromClass` "/Game/BluePrint/Hand/BP_Hand.BP_Hand_C" (`KismetMathLibrary.MakeTransform` (0.0 0.0 0.0)) "AlwaysSpawn" "MultiplyWithRoot" self true null))
          (bind _output_get_2 (set `self.LeftHand` _returnvalue_2))
          (`self.K2_AttachToComponent` _output_get_2 (`self.VRRoot`) "None" "SnapToTarget" "SnapToTarget" "KeepWorld" true))))
    (:`then_3`
      (if _istest
        (bind _returnvalue_3 (`|SpawnActorFromClass` "/Game/BluePrint/Hand/BP_Hand.BP_Hand_C" (`KismetMathLibrary.MakeTransform` (100.0 0.0 0.0) (struct :`Pitch` -90.0 :`Roll` -90.0)) "AlwaysSpawn" "MultiplyWithRoot" self false null))
        (bind _output_get_3 (set `self.RightHand` _returnvalue_3))
        (`self.K2_AttachToComponent` _output_get_3 (`self.VRRoot`) "None" "KeepRelative" "SnapToTarget" "KeepWorld" true)
        (else
          (bind _returnvalue_4 (`|SpawnActorFromClass` "/Game/BluePrint/Hand/BP_Hand.BP_Hand_C" (`KismetMathLibrary.MakeTransform` (0.0 0.0 0.0)) "AlwaysSpawn" "MultiplyWithRoot" self false null))
          (bind _output_get_4 (set `self.RightHand` _returnvalue_4))
          (`self.K2_AttachToComponent` _output_get_4 (`self.VRRoot`) "None" "SnapToTarget" "SnapToTarget" "KeepWorld" true))))))

(event `self.ReceiveTick`
  (params (DeltaSeconds :type "Float (single-precision)")))

(event `EnhancedInput|/Game/BluePrint/Input/InputAction/IA_VR_Move`
  (params (ActionValue :type "Float (double-precision)") (ElapsedSeconds :type "Float (double-precision)") (TriggeredSeconds :type "Float (double-precision)") (InputAction :type "InputAction Object Reference" :default "/Game/BluePrint/Input/InputAction/IA_VR_Move.IA_VR_Move"))
  (bind (_returnvalue_x _returnvalue_y) (`KismetMathLibrary.BreakVector` (`SceneComponent.GetForwardVector` (`self.Camera`))))
  ;[1 1 1] 카메라 기준으로 전진
  (:`Triggered`
    (`self.AddMovementInput` (`KismetMathLibrary.MakeVector` _returnvalue_x _returnvalue_y) ActionValue)))

(event `EnhancedInput|/Game/BluePrint/Input/InputAction/IA_VR_Trun`
  (params (ActionValue :type "Float (double-precision)") (ElapsedSeconds :type "Float (double-precision)") (TriggeredSeconds :type "Float (double-precision)") (InputAction :type "InputAction Object Reference" :default "/Game/BluePrint/Input/InputAction/IA_VR_Trun.IA_VR_Trun"))
  ;[1 1 1] 입력이 들어오면 스냅을 줘서 그때 한번씩 꺽는다
  (:`Started`
    (`self.SnapTurn` (> ActionValue 0.0))))

(event `EnhancedInput|/Game/BluePrint/Input/InputAction/IA_VR_Grab_Left`
  (params (ActionValue :type "Float (double-precision)") (ElapsedSeconds :type "Float (double-precision)") (TriggeredSeconds :type "Float (double-precision)") (InputAction :type "InputAction Object Reference" :default "/Game/BluePrint/Input/InputAction/IA_VR_Grab_Left.IA_VR_Grab_Left"))
  (bind _lefthand (`self.LeftHand`))
  (:`Started`
    (`/Game/BluePrint/Hand/BP_Hand.Handle Grab` _lefthand)
    (`KismetSystemLibrary.PrintString` "Left Handle Grab"))
  (:`Completed`
    (`/Game/BluePrint/Hand/BP_Hand.HandleRelease` _lefthand)
    (`KismetSystemLibrary.PrintString` "Left Handle Release")))

(event `EnhancedInput|/Game/BluePrint/Input/InputAction/IA_VR_Grab_Right`
  (params (ActionValue :type "Float (double-precision)") (ElapsedSeconds :type "Float (double-precision)") (TriggeredSeconds :type "Float (double-precision)") (InputAction :type "InputAction Object Reference" :default "/Game/BluePrint/Input/InputAction/IA_VR_Grab_Right.IA_VR_Grab_Right"))
  (bind _righthand (`self.RightHand`))
  (:`Started`
    (`/Game/BluePrint/Hand/BP_Hand.Handle Grab` _righthand)
    (`KismetSystemLibrary.PrintString` "Right Handle Grab"))
  (:`Completed`
    (`/Game/BluePrint/Hand/BP_Hand.HandleRelease` _righthand)
    (`KismetSystemLibrary.PrintString` "Right Handle Release")))

(fn `SnapTurn`
  (params (RIghtTurn :type Boolean))
  (locals (LocalPrevCameraLocation :type "Vector Structure" :default (0.0 0.0 0.0)))
  (bind _snapturndegree (`self.SnapTurnDegree`))
  (bind _returnvalue (- (`local.LocalPrevCameraLocation`) (`SceneComponent.K2_GetComponentLocation` (`self.Camera`))))
  ;[1 1 1] 돌기 전 카메라 위치
  (set `local.LocalPrevCameraLocation` (`SceneComponent.K2_GetComponentLocation` (`self.Camera`)))
  (`self.K2_AddActorWorldRotation` (`KismetMathLibrary.MakeRotator` 0.0 0.0 (`KismetMathLibrary.SelectFloat` (`KismetMathLibrary.Abs` _snapturndegree) _snapturndegree (`local.RIghtTurn`))))
  ;[1 1 1] 카메라의 상대 트랜스폼을 따라가지고 옵셋을 더해준다(카메라 회전시 생기는 오차를 보정해준다
  (`self.K2_AddActorWorldOffset` _returnvalue false true)
  (`KismetSystemLibrary.PrintText` (`KismetTextLibrary.Conv_DoubleToText` (.z _returnvalue) "HalfToEven")))

(fn `UserConstructionScript`)