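; BP_Hand is an XR hand actor that serves as either the left or right hand, chosen by the IsLeftHand flag.
; The Construction Script assigns the matching MannyXR skeletal mesh and rotation to HandMesh.
; BeginPlay assigns the mesh again, applies a different yaw from the Construction Script's, and sets the MotionController's motion source to Left or Right.
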(event `self.ReceiveBeginPlay`
  (bind _handmesh (`self.HandMesh`))
  (bind _handmesh_2 (`self.HandMesh`))
  (bind _motioncontroller (`self.MotionController`))
  (if (`self.IsLeftHand`)
    (`SkeletalMeshComponent.SetSkeletalMeshAsset` _handmesh_2 "/Game/VRFramework/Characters/MannequinsXR/Meshes/SKM_MannyXR_left.SKM_MannyXR_left")
    (`SceneComponent.K2_SetRelativeRotation` _handmesh (struct :`Pitch` -25.0 :`Roll` -90.0) false false)
    (set `MotionControllerComponent.MotionSource` "Left" _motioncontroller)
    (else
      (`SkeletalMeshComponent.SetSkeletalMeshAsset` _handmesh_2 "/Game/VRFramework/Characters/MannequinsXR/Meshes/SKM_MannyXR_right.SKM_MannyXR_right")
      (`SceneComponent.K2_SetRelativeRotation` _handmesh (struct :`Pitch` 25.0 :`Roll` 90.0) false false)
      (set `MotionControllerComponent.MotionSource` "Right" _motioncontroller))))

(fn `UserConstructionScript`
  (bind _handmesh (`self.HandMesh`))
  (bind _handmesh_2 (`self.HandMesh`))
  (if (`self.IsLeftHand`)
    (`SkeletalMeshComponent.SetSkeletalMeshAsset` _handmesh_2 "/Game/VRFramework/Characters/MannequinsXR/Meshes/SKM_MannyXR_left.SKM_MannyXR_left")
    (`SceneComponent.K2_SetRelativeRotation` _handmesh (struct :`Pitch` -90.0 :`Roll` -90.0) false false)
    (else
      (`SkeletalMeshComponent.SetSkeletalMeshAsset` _handmesh_2 "/Game/VRFramework/Characters/MannequinsXR/Meshes/SKM_MannyXR_right.SKM_MannyXR_right")
      (`SceneComponent.K2_SetRelativeRotation` _handmesh (struct :`Pitch` 90.0 :`Roll` 90.0) false false))))