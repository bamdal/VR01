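; VR player character that handles camera-relative movement, snap turning, two-handed grabbing and a toggleable menu through Enhanced Input.
; BeginPlay adds the mapping context, shifts VRRoot to the desired camera height after a short delay, and spawns left and right BP_Hand actors attached to it.
; Grab inputs forward to each hand, while either menu input spawns or closes BP_Menu.
; An IsTest flag alters hand placement, prints grab messages and passes to hands and menu.
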(event `EnhancedInput|/Game/BluePrint/Input/InputAction/IA_VR_Move`
  (params (ActionValue :type "Float (double-precision)") (ElapsedSeconds :type "Float (double-precision)") (TriggeredSeconds :type "Float (double-precision)") (InputAction :type "InputAction Object Reference" :default "/Game/BluePrint/Input/InputAction/IA_VR_Move.IA_VR_Move"))
  (bind (_returnvalue_x _returnvalue_y) (`KismetMathLibrary.BreakVector` (`SceneComponent.GetForwardVector` (`self.Camera`))))
  ;[1 1 1] 카메라 기준으로 전진
  (:`Triggered`
    (if (not (`self.Hit Wall`))
      (`self.AddMovementInput` (`KismetMathLibrary.MakeVector` _returnvalue_x _returnvalue_y) ActionValue))))

(event `self.ReceiveBeginPlay`
  (bind _istest (`self.IsTest`))
  (bind _istest_2 (`self.IsTest`))
  (bind (_returnvalue_x _returnvalue_y _returnvalue_z) (`KismetMathLibrary.BreakVector` (`SceneComponent.K2_GetComponentLocation` (`self.Camera`))))
  (`|ExecutionSequence`
    (:`then_0`
      ;[1 1 1] Input Mapping Context
      (`EnhancedInputSubsystemInterface.AddMappingContext` (pcsubsystem `EnhancedInputLocalPlayerSubsystem` (`GameplayStatics.GetPlayerController` 0)) "/Game/BluePrint/Input/IMC_VR_Default.IMC_VR_Default" 0 (struct)))
    (:`then_1`
      ;[1 1 1] 원하는 시작위치로 VRRoot를 보정하여 시작할 수 있어야 한다
      (`HeadMountedDisplayFunctionLibrary.SetTrackingOrigin` "View")
      (`KismetSystemLibrary.Delay` 0.2) ; 물리 시간 보정용 delay
      (`SceneComponent.K2_AddRelativeLocation` (`self.VRRoot`) (`KismetMathLibrary.MakeVector` 0.0 0.0 (- (`self.DesiredCameraHeight`) _returnvalue_z)) false false))
    (:`then_2`
      (if _istest
        (bind _returnvalue (`|SpawnActorFromClass` "/Game/BluePrint/Hand/BP_Hand.BP_Hand_C" (`KismetMathLibrary.MakeTransform` (100.0 0.0 0.0) (struct :`Pitch` 90.0 :`Roll` 90.0)) "AlwaysSpawn" "MultiplyWithRoot" self true null))
        (set `/Game/BluePrint/Hand/BP_Hand.IsTest` (`self.IsTest`) _returnvalue)
        (bind _output_get (set `self.LeftHand` _returnvalue))
        (`self.K2_AttachToComponent` _output_get (`self.VRRoot`) "None" "KeepRelative" "SnapToTarget" "KeepWorld" true)
        (else
          ;[1 1 1] Make Hand
          (bind _returnvalue_2 (`|SpawnActorFromClass` "/Game/BluePrint/Hand/BP_Hand.BP_Hand_C" (`KismetMathLibrary.MakeTransform` (0.0 0.0 0.0)) "AlwaysSpawn" "MultiplyWithRoot" self true null))
          (bind _output_get_2 (set `self.LeftHand` _returnvalue_2))
          (`self.K2_AttachToComponent` _output_get_2 (`self.VRRoot`) "None" "SnapToTarget" "SnapToTarget" "KeepWorld" true))))
    (:`then_3`
      (if _istest
        (bind _returnvalue_3 (`|SpawnActorFromClass` "/Game/BluePrint/Hand/BP_Hand.BP_Hand_C" (`KismetMathLibrary.MakeTransform` (100.0 0.0 0.0) (struct :`Pitch` -90.0 :`Roll` -90.0)) "AlwaysSpawn" "MultiplyWithRoot" self false null))
        (set `/Game/BluePrint/Hand/BP_Hand.IsTest` (`self.IsTest`) _returnvalue_3)
        (bind _output_get_3 (set `self.RightHand` _returnvalue_3))
        (`self.K2_AttachToComponent` _output_get_3 (`self.VRRoot`) "None" "KeepRelative" "SnapToTarget" "KeepWorld" true)
        (else
          (bind _returnvalue_4 (`|SpawnActorFromClass` "/Game/BluePrint/Hand/BP_Hand.BP_Hand_C" (`KismetMathLibrary.MakeTransform` (0.0 0.0 0.0)) "AlwaysSpawn" "MultiplyWithRoot" self false null))
          (bind _output_get_4 (set `self.RightHand` _returnvalue_4))
          (`self.K2_AttachToComponent` _output_get_4 (`self.VRRoot`) "None" "SnapToTarget" "SnapToTarget" "KeepWorld" true))))
    (:`then_4`
      (`/Game/BluePrint/Hand/BP_Hand.SpawnHand` (`self.LeftHand`) _istest_2)
      (`/Game/BluePrint/Hand/BP_Hand.SpawnHand` (`self.RightHand`) _istest_2))))

(event `EnhancedInput|/Game/BluePrint/Input/InputAction/IA_VR_Trun`
  (params (ActionValue :type "Float (double-precision)") (ElapsedSeconds :type "Float (double-precision)") (TriggeredSeconds :type "Float (double-precision)") (InputAction :type "InputAction Object Reference" :default "/Game/BluePrint/Input/InputAction/IA_VR_Trun.IA_VR_Trun"))
  ;[1 1 1] 입력이 들어오면 스냅을 줘서 그때 한번씩 꺽는다
  (:`Started`
    (`self.SnapTurn` (> ActionValue 0.1))))

(event `EnhancedInput|/Game/BluePrint/Input/InputAction/IA_VR_Grab_Left`
  (params (ActionValue :type "Float (double-precision)") (ElapsedSeconds :type "Float (double-precision)") (TriggeredSeconds :type "Float (double-precision)") (InputAction :type "InputAction Object Reference" :default "/Game/BluePrint/Input/InputAction/IA_VR_Grab_Left.IA_VR_Grab_Left"))
  (bind _lefthand (`self.LeftHand`))
  ;[1 1 1] Grab event
  (:`Started`
    (`/Game/BluePrint/Hand/BP_Hand.Handle Grab` _lefthand)
    (if (`self.IsTest`)
      (`KismetSystemLibrary.PrintString` "Left Handle Grab")))
  (:`Completed`
    (`/Game/BluePrint/Hand/BP_Hand.HandleRelease` _lefthand)
    (if (`self.IsTest`)
      (`KismetSystemLibrary.PrintString` "Left Handle Release"))))

(event `EnhancedInput|/Game/BluePrint/Input/InputAction/IA_VR_Grab_Right`
  (params (ActionValue :type "Float (double-precision)") (ElapsedSeconds :type "Float (double-precision)") (TriggeredSeconds :type "Float (double-precision)") (InputAction :type "InputAction Object Reference" :default "/Game/BluePrint/Input/InputAction/IA_VR_Grab_Right.IA_VR_Grab_Right"))
  (bind _righthand (`self.RightHand`))
  ;[1 1 1] Grab event
  (:`Started`
    (`/Game/BluePrint/Hand/BP_Hand.Handle Grab` _righthand)
    (if (`self.IsTest`)
      (`KismetSystemLibrary.PrintString` "Right Handle Grab")))
  (:`Completed`
    (`/Game/BluePrint/Hand/BP_Hand.HandleRelease` _righthand)
    (if (`self.IsTest`)
      (`KismetSystemLibrary.PrintString` "Right Handle Release"))))

(event `EnhancedInput|/Game/BluePrint/Input/InputAction/IA_VR_Menu_Toggle_Left`
  (params (ActionValue :type Boolean) (ElapsedSeconds :type "Float (double-precision)") (TriggeredSeconds :type "Float (double-precision)") (InputAction :type "InputAction Object Reference" :default "/Game/BluePrint/Input/InputAction/IA_VR_Menu_Toggle_Left.IA_VR_Menu_Toggle_Left"))
  ;[1 1 1] 메뉴 활성화
  (:`Started`
    (`self.ToggleMenu` :!label _label)))

(event `EnhancedInput|/Game/BluePrint/Input/InputAction/IA_VR_Menu_Toggle_Right`
  (params (ActionValue :type Boolean) (ElapsedSeconds :type "Float (double-precision)") (TriggeredSeconds :type "Float (double-precision)") (InputAction :type "InputAction Object Reference" :default "/Game/BluePrint/Input/InputAction/IA_VR_Menu_Toggle_Right.IA_VR_Menu_Toggle_Right"))
  ;[1 1 1] 메뉴 활성화
  (:`Started`
    (goto _label)))

(event `self.CapsuleComponent.OnComponentHit`
  (params (HitComponent :type "PrimitiveComponent Object Reference") (OtherActor :type "Actor Object Reference") (OtherComp :type "PrimitiveComponent Object Reference") (NormalImpulse :type "Vector Structure") (Hit :type "HitResult Structure (by ref)"))
  (switch `ECollisionChannel` (`PrimitiveComponent.GetCollisionObjectType` OtherComp)))

(fn `SnapTurn`
  (params (RIghtTurn :type Boolean))
  (locals (LocalPrevCameraLocation :type "Vector Structure" :default (0.0 0.0 0.0)))
  (bind _snapturndegree (`self.SnapTurnDegree`))
  (bind _returnvalue (`KismetMathLibrary.SelectFloat` (`KismetMathLibrary.Abs` _snapturndegree) _snapturndegree (`local.RIghtTurn`)))
  ;[1 1 1] 돌기 전 카메라 위치
  (set `local.LocalPrevCameraLocation` (`SceneComponent.K2_GetComponentLocation` (`self.Camera`)))
  (`self.AddControllerYawInput` _returnvalue)
  (`self.K2_AddActorWorldRotation` (`KismetMathLibrary.MakeRotator` 0.0 0.0 _returnvalue)))

(fn `ToggleMenu`
  (`/Engine/EditorBlueprintResources/StandardMacros.IsValid` (`self.MenuReference`)
    (:`Is Valid`
      (`/Game/BluePrint/UI/BP_Menu.CloseMenu` (`self.MenuReference`))
      (set `self.MenuReference` null))
    (:`Is Not Valid`
      (bind _returnvalue (`|SpawnActorFromClass` "/Game/BluePrint/UI/BP_Menu.BP_Menu_C" (`KismetMathLibrary.MakeTransform` (+ (`self.K2_GetActorLocation`) (* (`self.GetActorForwardVector`) 500.0))) "Undefined" "MultiplyWithRoot" null self))
      (set `/Game/BluePrint/UI/BP_Menu.IsTest` (`self.IsTest`) _returnvalue)
      (set `self.MenuReference` _returnvalue))))

(fn `UserConstructionScript`)