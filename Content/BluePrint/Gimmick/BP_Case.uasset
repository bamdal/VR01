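; BP_Case is a VR gimmick actor that a player grabs and slides along its own forward axis, like a case or drawer.
; On grab, it stores the actor and motion controller start locations from the grab component's hand.
; While held, Tick projects the controller's total displacement since grab onto the forward vector and adds it to the start location.
; Two per-frame delta variants remain unconnected.
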(event `self.BP_GrabComponent.Grabbed`
  (bind _motioncontroller (`self.GetMotionController`))
  (`/Engine/EditorBlueprintResources/StandardMacros.IsValid` _motioncontroller
    (:`Is Valid`
      (bind _output_get (set `self.MCGrabLocation` (`SceneComponent.K2_GetComponentLocation` _motioncontroller)))
      (set `self.PreMCGrabLocation` _output_get)
      (set `self.ActorGrabLocation` (`self.K2_GetActorLocation`))
      (set `self.Grabed` true))))

(event `self.BP_GrabComponent.OnDrop`
  (set `self.Grabed` false))

(event `self.ReceiveTick`
  (params (DeltaSeconds :type "Float (single-precision)"))
  (bind _motioncontroller (`self.GetMotionController`))
  (if (`self.Grabed`)
    ;[1 1 1] 초기 위치 저장 후, 마지막 위치 - 초기 위치 차이 계산
    (`/Engine/EditorBlueprintResources/StandardMacros.IsValid` _motioncontroller
      (:`Is Valid`
        (`self.K2_SetActorLocation` (+ (`KismetMathLibrary.ProjectVectorOnToVector` (- (`SceneComponent.K2_GetComponentLocation` _motioncontroller) (`self.MCGrabLocation`)) (`self.GetActorForwardVector`)) (`self.ActorGrabLocation`)) false true)))))

(fn `GetMotionController`
  (returns (MotionController :type "MotionControllerComponent Object Reference"))
  (bind _grabbinghand (`/Game/BluePrint/BP_GrabComponent.GrabbingHand` (`self.BP_GrabComponent`)))
  (`/Engine/EditorBlueprintResources/StandardMacros.IsValid` _grabbinghand
    (:`Is Valid`
      (return (`/Game/BluePrint/Hand/BP_Hand.MotionController` _grabbinghand)))
    (:`Is Not Valid`
      (return null))))

(fn `UserConstructionScript`)