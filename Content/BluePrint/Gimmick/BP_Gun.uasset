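; BP_Gun is a grabbable VR gun that fires projectiles from its muzzle with the hand holding it.
; Grab and drop events from the grab component toggle input and add or remove the left or right weapon mapping context.
; Each hand's shoot input checks the grabbing hand, then shares one path that spawns a projectile and plays a shot sound.
; Spawning ignores collisions so a muzzle close to the gun cannot block it.
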(event `self.BP_GrabComponent.Grabbed`
  (bind _returnvalue (`GameplayStatics.GetPlayerController` 0))
  ;[1 1 1] 총 획득 여부에 따라IMC 추가 삭제
  (`self.EnableInput` _returnvalue null)
  (`EnhancedInputSubsystemInterface.AddMappingContext` (pcsubsystem `EnhancedInputLocalPlayerSubsystem` _returnvalue) (select `bool` (`|EnumEquality` (`/Game/BluePrint/BP_GrabComponent.GetGrabbingHandType` (`self.BP_GrabComponent`)) "Left") :`false` "/Game/BluePrint/Input/IMC_VR_Weapon_Right.IMC_VR_Weapon_Right" :`true` "/Game/BluePrint/Input/IMC_VR_Weapon_Left.IMC_VR_Weapon_Left" :!type "InputMappingContext Object Reference") 0 (struct)))

(event `self.BP_GrabComponent.OnDrop`
  (bind _returnvalue (`GameplayStatics.GetPlayerController` 0))
  ;[1 1 1] 총 획득 여부에 따라IMC 추가 삭제
  (`self.DisableInput` _returnvalue null)
  (`EnhancedInputSubsystemInterface.RemoveMappingContext` (pcsubsystem `EnhancedInputLocalPlayerSubsystem` _returnvalue) (select `bool` (`|EnumEquality` (`/Game/BluePrint/BP_GrabComponent.GetGrabbingHandType` (`self.BP_GrabComponent`)) "Left") :`false` "/Game/BluePrint/Input/IMC_VR_Weapon_Right.IMC_VR_Weapon_Right" :`true` "/Game/BluePrint/Input/IMC_VR_Weapon_Left.IMC_VR_Weapon_Left" :!type "InputMappingContext Object Reference") (struct)))

(event `EnhancedInput|/Game/BluePrint/Input/InputAction/IA_VR_Shoot_Left`
  (params (ActionValue :type "Float (double-precision)") (ElapsedSeconds :type "Float (double-precision)") (TriggeredSeconds :type "Float (double-precision)") (InputAction :type "InputAction Object Reference" :default "/Game/BluePrint/Input/InputAction/IA_VR_Shoot_Left.IA_VR_Shoot_Left"))
  (bind _muzzlelocation (`self.MuzzleLocation`))
  ;[1 1 1] 총 발사
  (:`Started`
    (if (`|EnumEquality` (`/Game/BluePrint/BP_GrabComponent.GetGrabbingHandType` (`self.BP_GrabComponent`)) "Left")
      ;;[1 1 1] Projectile이 muzzle이 총과 가까우면 바로 충돌이 생겨서 스폰이 안됨
      (`|SpawnActorFromClass` "/Game/VRFramework/VRTemplate/Blueprints/Projectile.Projectile_C" (`KismetMathLibrary.MakeTransform` (`SceneComponent.K2_GetComponentLocation` _muzzlelocation) (`SceneComponent.K2_GetComponentRotation` _muzzlelocation)) "AlwaysSpawn" "OverrideRootScale" self (`GameplayStatics.GetPlayerPawn` 0) :!label _label)
      (`GameplayStatics.PlaySoundAtLocation` "/Engine/VREditor/Sounds/UI/Camera_Shutter.Camera_Shutter" (`SceneComponent.K2_GetComponentLocation` (`self.MuzzleLocation`)) (struct) 1.0 1.0 0.0 null null null null))))

(event `EnhancedInput|/Game/BluePrint/Input/InputAction/IA_VR_Shoot_RIght`
  (params (ActionValue :type "Float (double-precision)") (ElapsedSeconds :type "Float (double-precision)") (TriggeredSeconds :type "Float (double-precision)") (InputAction :type "InputAction Object Reference" :default "/Game/BluePrint/Input/InputAction/IA_VR_Shoot_RIght.IA_VR_Shoot_RIght"))
  ;[1 1 1] 총 발사
  (:`Started`
    (if (`|EnumEquality` (`/Game/BluePrint/BP_GrabComponent.GetGrabbingHandType` (`self.BP_GrabComponent`)) "Right")
      (goto _label))))

(fn `UserConstructionScript`)