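; BP_Cell_Door is a gimmick cell door that moves vertically to open and close.
; OpenDoor and CloseDoor, bound to matching event dispatchers at BeginPlay, set IsOpen and play or reverse the ToggleDoor timeline.
; The timeline drives the actor's relative Z directly, keeping X and Y from the mesh's starting world location.
; The 5 key flips the door through ToogleDoor based on IsOpen.
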(event `self.ReceiveBeginPlay`
  (set `self.StartLocation` (`SceneComponent.K2_GetComponentLocation` (`self.StaticMeshComponent`)))
  (add `self.OpenDoorEvent` (delegate `OpenDoor`))
  (add `self.CloseDoorEvent` (delegate `CloseDoor`)))

(event `OpenDoorEvent_Event`
  (bind (_startlocation_x _startlocation_y) (`KismetMathLibrary.BreakVector` (`self.StartLocation`)))
  (set `self.IsOpen` true :!label _label)
  (bind (_direction _return_value) (`Timeline|ToggleDoor` :!label _label_2)
    (:`Update`
      (`self.K2_SetActorRelativeLocation` (`KismetMathLibrary.MakeVector` _startlocation_x _startlocation_y _return_value)))))

(event `OpenDoor`
  (goto _label))

(event `CloseDoorEvent_Event`
  (set `self.IsOpen` false :!label _label_3)
  (goto _label_2 :!via `Reverse`))

(event `CloseDoor`
  (goto _label_3))

(event `ToogleDoor`
  (if (`self.IsOpen`)
    (`self.CloseDoor`)
    (else
      (`self.OpenDoor`))))

(event `Key|Five`
  (params (Key :type "Key Structure"))
  (:`Pressed`
    (`self.ToogleDoor`)))

(fn `UserConstructionScript`)