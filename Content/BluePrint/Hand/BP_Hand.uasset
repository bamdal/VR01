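; BP_Hand is a VR hand actor for left or right that picks up and drops objects carrying a BP_GrabComponent.
; SpawnHand sets mesh, rotation and motion source per side, with a separate test orientation, then caches the mesh transform for ResetHandMesh to restore.
; HandleGrab poses ABP_Hand and sphere-traces at the motion controller for a grab component to hold.
; HandleRelease drops it and opens the hand.
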(event `self.ReceiveBeginPlay`)

(event `SpawnHand`
  (params (isTest :type Boolean))
  (bind _handmesh (`self.HandMesh`))
  (bind _motioncontroller (`self.MotionController`))
  (bind _handmesh_2 (`self.HandMesh`))
  (bind _motioncontroller_2 (`self.MotionController`))
  (bind _handmesh_3 (`self.HandMesh`))
  (bind _handmesh_4 (`self.HandMesh`))
  (set `self.IsTest` isTest)
  (`|ExecutionSequence`
    (:`then_0`
      ;[1 1 1] Test 용
      (if (`self.IsTest`)
        (if (`self.IsLeftHand`)
          (`SkeletalMeshComponent.SetSkeletalMeshAsset` _handmesh_2 "/Game/VRFramework/Characters/MannequinsXR/Meshes/SKM_MannyXR_left.SKM_MannyXR_left")
          (`SceneComponent.K2_SetRelativeRotation` _handmesh (struct :`Yaw` -90.0) false false)
          (set `MotionControllerComponent.MotionSource` "Left" _motioncontroller_2)
          (else
            (`SkeletalMeshComponent.SetSkeletalMeshAsset` _handmesh_2 "/Game/VRFramework/Characters/MannequinsXR/Meshes/SKM_MannyXR_right.SKM_MannyXR_right")
            (`SceneComponent.K2_SetRelativeRotation` _handmesh (struct :`Yaw` -90.0) false false)
            (set `MotionControllerComponent.MotionSource` "Right" _motioncontroller_2)))
        (elif (`self.IsLeftHand`)
          (`SkeletalMeshComponent.SetSkeletalMeshAsset` _handmesh_3 "/Game/VRFramework/Characters/MannequinsXR/Meshes/SKM_MannyXR_left.SKM_MannyXR_left")
          (`SceneComponent.K2_SetRelativeRotation` _handmesh_4 (struct :`Pitch` -115.0 :`Roll` -90.0) false false)
          (set `MotionControllerComponent.MotionSource` "Left" _motioncontroller)
          (else
            (`SkeletalMeshComponent.SetSkeletalMeshAsset` _handmesh_3 "/Game/VRFramework/Characters/MannequinsXR/Meshes/SKM_MannyXR_right.SKM_MannyXR_right")
            (`SceneComponent.K2_SetRelativeRotation` _handmesh_4 (struct :`Pitch` 25.0 :`Roll` 90.0) false false)
            (set `MotionControllerComponent.MotionSource` "Right" _motioncontroller)))))
    (:`then_1`
      (set `self.InitHandMeshRelativeTransform` (`SceneComponent.GetRelativeTransform` (`self.HandMesh`))))))

(fn `FindGrabComponentNearHand`
  (returns (GrabComponent :type "/Game/BluePrint/BP_GrabComponent Object Reference"))
  (locals (LocalGrabComponent :type "/Game/BluePrint/BP_GrabComponent Object Reference") (LocalGripPosition :type "Vector Structure" :default (0.0 0.0 0.0)))
  (`|ExecutionSequence`
    (:`then_0`
      ;[1 1 1] GrabComponent 찾기
      (bind _output_get (set `local.LocalGripPosition` (`SceneComponent.K2_GetComponentLocation` (`self.MotionController`))))
      (bind (_outhit _returnvalue) (`KismetSystemLibrary.SphereTraceSingleForObjects` :`Start` _output_get :`End` _output_get :`Radius` (`self.Radius`) :`ObjectTypes` (`|MakeArray` "ObjectTypeQuery7" :!type "EObjectTypeQuery Enum") :`DrawTime` 1.0)) ; motion controller의 위치에서 찾기
      (if _returnvalue
        (bind _returnvalue_2 (`self.GetComponentByClass` (`.HitActor` (`GameplayStatics.BreakHitResult` _outhit)) "/Game/BluePrint/BP_GrabComponent.BP_GrabComponent_C"))
        (`/Engine/EditorBlueprintResources/StandardMacros.IsValid` _returnvalue_2
          (:`Is Valid`
            (set `local.LocalGrabComponent` _returnvalue_2)))))
    (:`then_1`
      (return (`local.LocalGrabComponent`)))))

(fn `Handle Grab`
  (`|ExecutionSequence`
    (:`then_0`
      ;[1 1 1] 잡는 애니메이션
      (bind _asabp_hand (cast `/Game/BluePrint/Hand/ABP_Hand` (`SkeletalMeshComponent.GetAnimInstance` (`self.HandMesh`))))
      (set `/Game/BluePrint/Hand/ABP_Hand.Mirror` (`self.IsLeftHand`) _asabp_hand)
      (set `/Game/BluePrint/Hand/ABP_Hand.PoseAlphaGrab` 1.0 _asabp_hand))
    (:`then_1`
      ;[1 1 1] 잡는 연산 시작
      (bind _grabcomponent (`self.FindGrabComponentNearHand`))
      (`/Engine/EditorBlueprintResources/StandardMacros.IsValid` _grabcomponent
        (:`Is Valid`
          (bind _gethand (`/Game/BluePrint/BP_GrabComponent.TryGrab` _grabcomponent self))
          (if _gethand
            (set `self.HeldComponent` _grabcomponent)
            (`/Game/BluePrint/BP_GrabComponent.Grabbed` _grabcomponent)))))))

(fn `HandleRelease`
  (bind _heldcomponent (`self.HeldComponent`))
  (`|ExecutionSequence`
    (:`then_0`
      (`/Engine/EditorBlueprintResources/StandardMacros.IsValid` _heldcomponent
        (:`Is Valid`
          (`/Game/BluePrint/BP_GrabComponent.OnDrop` _heldcomponent)
          (`/Game/BluePrint/BP_GrabComponent.TryRelease` _heldcomponent))))
    (:`then_1`
      ;[1 1 1] 손을 펴는 애니매이션
      (bind _asabp_hand (cast `/Game/BluePrint/Hand/ABP_Hand` (`SkeletalMeshComponent.GetAnimInstance` (`self.HandMesh`))))
      (set `/Game/BluePrint/Hand/ABP_Hand.Mirror` (`self.IsLeftHand`) _asabp_hand)
      (set `/Game/BluePrint/Hand/ABP_Hand.PoseAlphaGrab` 0.0 _asabp_hand))))

(fn `ResetHandMesh`
  (`SceneComponent.K2_AttachToComponent` (`self.HandMesh`) (`self.MotionController`) "None" "KeepRelative" "KeepRelative" "KeepRelative" true)
  (`SceneComponent.K2_SetRelativeTransform` (`self.HandMesh`) (`self.InitHandMeshRelativeTransform`) false true))

(fn `UserConstructionScript`
  (bind _handmesh (`self.HandMesh`))
  (bind _handmesh_2 (`self.HandMesh`))
  (if (`self.IsLeftHand`)
    (`SkeletalMeshComponent.SetSkeletalMeshAsset` _handmesh_2 "/Game/VRFramework/Characters/MannequinsXR/Meshes/SKM_MannyXR_left.SKM_MannyXR_left")
    (`SceneComponent.K2_SetRelativeRotation` _handmesh (struct :`Pitch` -90.0 :`Roll` -90.0) false false)
    (else
      (`SkeletalMeshComponent.SetSkeletalMeshAsset` _handmesh_2 "/Game/VRFramework/Characters/MannequinsXR/Meshes/SKM_MannyXR_right.SKM_MannyXR_right")
      (`SceneComponent.K2_SetRelativeRotation` _handmesh (struct :`Pitch` 90.0 :`Roll` 90.0) false false))))